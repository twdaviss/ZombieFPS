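; Zombie spawner actor that releases escalating waves of BP_Zombie AI pawns around its own location.
; Tick accumulates a timer and, once it exceeds the spawn delay, spawns the current batch at small random horizontal offsets using the spawner's rotation.
; After each wave the timer resets, the batch grows by one, and the delay shrinks only slightly, by a fraction of that frame's delta time.
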(event `self.ReceiveTick`
  (params (DeltaSeconds :type "Float (single-precision)"))
  (bind _returnvalue (`self.GetTransform`))
  (if (> (`self.spawnDelayTimer`) (`self.SpawnDelay`))
    (for _ (range 1 (+ (`self.SpawnAmount`) 1))
      (`AIBlueprintHelperLibrary.SpawnAIFromClass` "/Game/ZombieFPS/BP_Zombie.BP_Zombie_C" null (`KismetMathLibrary.MakeVector` (+ (`KismetMathLibrary.RandomIntegerInRange` -50 50) (.x (.location _returnvalue))) (+ (`KismetMathLibrary.RandomIntegerInRange` -50 50) (.y (.location _returnvalue))) (.z (.location _returnvalue))) (.rotation _returnvalue) false null))
    (set `self.spawnDelayTimer` 0.0)
    (set `self.spawnDelay` (- (`self.spawnDelay`) (* DeltaSeconds 0.1)))
    (`/Engine/EditorBlueprintResources/StandardMacros.IncrementInt` (`self.spawnAmount`))
    (else
      (set `self.spawnDelayTimer` (+ DeltaSeconds (`self.spawnDelayTimer`))))))

(fn `UserConstructionScript`)