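; BP_Zombie is an enemy character that chases the first player and deals melee damage.
; Tick re-issues an AI MoveTo toward the player while it can attack; reaching them applies damage, then starts a one-second cooldown.
; Incoming damage lowers health and briefly staggers it by disabling movement.
; When health drops below zero, Tick destroys the zombie and adds its points to the first-person game mode's score.
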(event `self.ReceiveTick`
  (params (DeltaSeconds :type "Float (single-precision)"))
  (if (< (`self.currentHealth`) 0.0)
    (`self.K2_DestroyActor`)
    (bind _asbp_first_person_game_mode (cast `/Game/FirstPerson/Blueprints/BP_FirstPersonGameMode` (`GameplayStatics.GetGameMode`)))
    (set `/Game/FirstPerson/Blueprints/BP_FirstPersonGameMode.Points` (+ (`/Game/FirstPerson/Blueprints/BP_FirstPersonGameMode.Points` _asbp_first_person_game_mode) (`self.points`)) _asbp_first_person_game_mode)
    (else
      (`self.FollowPlayer`))))

(event `self.PawnSensing.OnSeePawn`
  (params (Pawn :type "Pawn Object Reference")))

(event `FollowPlayer`
  (bind _returnvalue (`GameplayStatics.GetPlayerCharacter` 0))
  (if (`self.canAttack`)
    (`|AIMoveTo` self (0.0 0.0 0.0) _returnvalue 100.0
      (:`OnSuccess`
        (if (`self.canAttack`)
          (set `self.canAttack` false)
          (set `self.attacking` true)
          (bind _asbp_first_person_character (cast `/Game/FirstPerson/Blueprints/BP_FirstPersonCharacter` _returnvalue))
          (`/Game/FirstPerson/Blueprints/BP_FirstPersonCharacter.DealDamage` _asbp_first_person_character (`self.damage`))
          (`KismetSystemLibrary.PrintString` "player hit")
          (`KismetSystemLibrary.Delay` 1.0)
          (set `self.canAttack` true)
          (set `self.attacking` false))))))

(event `DealDamage`
  (params (Damage :type "Float (double-precision)"))
  (bind _charactermovement (`self.CharacterMovement`))
  (set `self.currentHealth` (- (`self.currentHealth`) Damage))
  (set `self.staggered` true)
  (`CharacterMovementComponent.DisableMovement` _charactermovement)
  (`KismetSystemLibrary.Delay` 0.5)
  (set `self.staggered` false)
  (`CharacterMovementComponent.SetMovementMode` _charactermovement "MOVE_Walking" 0))

(fn `UserConstructionScript`)